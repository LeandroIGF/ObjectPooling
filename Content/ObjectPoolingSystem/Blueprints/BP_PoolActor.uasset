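; BP_PoolActor is a pooled actor that returns itself to the object pool shortly after activation.
; Activate calls the parent logic, then starts a one-second lifetime timer and stores its handle.
; When the timer fires, CE_DeactivateBP passes the actor and its class to ReturnProjectileToPool, while Deactivate only calls the parent logic.
; The construction script is empty, with unconnected leftover logic for attaching a box collider to the Cube.
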(event Custom|CE_DeactivateBP
  (bind _self self)
  (CallFunction|ReturnProjectiletoPool (Utilities|GetClass _self) _self))

(event EventBeginPlay)

(event Collision|EventActorBeginOverlap
  (params (OtherActor :type Actor%20Object%20Reference)))

(event EventTick
  (params (DeltaSeconds :type Float%20%28single-precision%29)))

(event EventDeactivate
  (|CallParentFunction))

(event EventActivate
  (params (ObjectPoolData :type Object%20Pool%20Activation%20Data%20Structure))
  (|CallParentFunction ObjectPoolData)
  (bind _returnvalue (Utilities|Time|SetTimerbyEvent (delegate Custom|CE_DeactivateBP) 1.0))
  (Variables|Default|SetDeactivateLifeTimerHandle _returnvalue))

(fn ConstructionScript)