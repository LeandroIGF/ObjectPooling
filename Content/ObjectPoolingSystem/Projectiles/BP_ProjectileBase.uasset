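; Base pooled projectile that moves forward with a swept offset every Tick and is reused through an object pool interface.
; Activate applies the pooled transform, restores collision and visibility, tints a cached dynamic material and starts a lifetime timer.
; A hit clears that timer and calls Deactivate, which returns the actor to the pool, hides it, disables collision and resets the color.
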(event EventTick
  (params (DeltaSeconds :type Float%20%28single-precision%29))
  ;[0.15 0.15 0.15 0.5] Simple projectile movement forward
  (Transformation|SetActorLocation (+ (Transformation|GetActorLocation) (* (Transformation|GetActorForwardVector) 1e+02 DeltaSeconds)) true false))

(event Collision|EventHit
  (params (MyComp :type Primitive%20Component%20Object%20Reference) (Other :type Actor%20Object%20Reference) (OtherComp :type Primitive%20Component%20Object%20Reference) (bSelfMoved :type Boolean) (HitLocation :type Vector :default "0, 0, 0") (HitNormal :type Vector :default "0, 0, 0") (NormalImpulse :type Vector :default "0, 0, 0") (Hit :type Hit%20Result%20Structure%20%28by%20ref%29))
  (Utilities|Time|ClearandInvalidateTimerbyHandle (Variables|Default|GetDeactivateLifeTimerHandle))
  (Class|ObjectPoolInterface|Deactivate))

(event Custom|Deactivate)

(event Custom|Activate)

(event EventActivate
  (params (ObjectPoolData :type Object%20Pool%20Activation%20Data%20Structure))
  ;[0.15 0.15 0.15 0.5] Setup Actor when activated
  (CallFunction|GameplaySetup ObjectPoolData)
  (CallFunction|VFXSetup)
  (bind _returnvalue (Utilities|Time|SetTimerbyEvent (EventDispatchers|CreateEvent :!event BPDeactivate) 6.0))
  (Variables|Default|SetDeactivateLifeTimerHandle _returnvalue))

(event EventDeactivate
  (bind _self self)
  (CallFunction|ReturnProjectiletoPool (Utilities|GetClass _self) _self)
  (Rendering|SetActorHiddenInGame true)
  (Collision|SetActorEnableCollision false)
  (Utilities|IsValid (Variables|Default|GetMID_Color)
    (:Is%20Valid
      (Rendering|Material|SetVectorParameterValue (Variables|Default|GetMID_Color) "Color" "(R=0.000000,G=0.031916,B=1.000000,A=1.000000)" :!class /Script/Engine.MaterialInstanceDynamic))))

(fn ConstructionScript)

(fn GameplaySetup
  (params (SetupData :type Object%20Pool%20Activation%20Data%20Structure))
  (Transformation|SetActorTransform (Utilities|Struct|BreakObjectPoolActivationData SetupData))
  (Collision|SetActorEnableCollision true)
  (Rendering|SetActorHiddenInGame false))

(fn VFXSetup
  (Utilities|IsValid (Variables|Default|GetMID_Color)
    (:Is%20Valid
      _)
    (:Is%20Not%20Valid
      (bind _returnvalue (Rendering|Material|CreateDynamicMaterialInstance (Variables|Default|GetSphere) 0 0 "None" :!class /Script/Engine.PrimitiveComponent))
      (Variables|Default|SetMID_Color _returnvalue)))
  (Rendering|Material|SetVectorParameterValue (Variables|Default|GetMID_Color) "Color" "(R=0.118656,G=1.000000,B=0.000000,A=1.000000)" :!class /Script/Engine.MaterialInstanceDynamic))