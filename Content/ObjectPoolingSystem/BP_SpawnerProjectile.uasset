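; BP_SpawnerProjectile is a spawner actor that emits pooled projectiles along its forward direction.
; On BeginPlay it creates an object pool for its ProjectileClass.
; Every Tick it takes a projectile from that pool and activates it with transform data placing it just ahead of the actor, facing forward at unit scale.
; It has no timer or fire-rate check, so it requests one projectile per frame.
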(event EventBeginPlay
  (CallFunction|CreateObjectPool (Variables|Default|GetProjectileClass)))

(event Collision|EventActorBeginOverlap
  (params (OtherActor :type Actor%20Object%20Reference)))

(event EventTick
  (params (DeltaSeconds :type Float%20%28single-precision%29))
  (bind _returnvalue (Transformation|GetActorForwardVector))
  (bind _objectpoolref (CallFunction|GetProjectilefromPool (Variables|Default|GetProjectileClass)))
  (bind _output_get (Variables|Default|SetObject%20Pool%20Activation%20Data (Utilities|Struct|MakeObjectPoolActivationData (Math|Transform|MakeTransform (+ (Transformation|GetActorLocation) (* _returnvalue 1e+02)) (Math|Rotator|MakeRotfromX _returnvalue) "1.000000,1.000000,1.000000"))))
  (Class|ObjectPoolInterface|Activate _objectpoolref _output_get))

(fn ConstructionScript)